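; A fixed-camera trigger Blueprint that switches the player's view to a referenced camera when a ThirdPersonCharacter enters its box.
; The box overlap blends player 0's view target to CamRef and registers it as that character's current camera.
; Every tick, CamRef's relative rotation is aimed at the player pawn using the direction vector between them, whether or not it is the active view.
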(event `self.Box.OnComponentBeginOverlap`
  (params (OverlappedComponent :type "PrimitiveComponent Object Reference") (OtherActor :type "Actor Object Reference") (OtherComp :type "PrimitiveComponent Object Reference") (OtherBodyIndex :type Integer) (bFromSweep :type Boolean) (SweepResult :type "HitResult Structure (by ref)"))
  (bind _asthird_person_character (cast `/Game/ThirdPersonBP/Blueprints/ThirdPersonCharacter` OtherActor))
  (`PlayerController.SetViewTargetWithBlend` (`GameplayStatics.GetPlayerController` 0) (`self.Cam_Ref`) 0.0 "VTBlend_Linear" 0.0 false)
  (`/Game/ThirdPersonBP/Blueprints/ThirdPersonCharacter.SetCurrentCam` _asthird_person_character (`self.Cam_Ref`)))

(event `self.ReceiveTick`
  (params (DeltaSeconds :type "Float (single-precision)"))
  (bind _cam_ref (`self.Cam_Ref`))
  (`self.K2_SetActorRelativeRotation` _cam_ref (`KismetMathLibrary.Conv_VectorToRotator` (- (`self.K2_GetActorLocation` (`GameplayStatics.GetPlayerPawn` 0)) (`self.K2_GetActorLocation` _cam_ref))) false false))

(fn `UserConstructionScript`)